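; BP_FallingPlatform is a platform that drops after BP_Brian steps into its trigger, then returns to where it started.
; Activation is guarded by a flag, stores the start transform and waits briefly before enabling physics for a timed fall.
; Reset disables physics and uses a timeline to lerp the platform back, then re-arms it.
; Each phase swaps the material and plays a sound, with debug text marking progress.
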(event OnComponentBeginOverlap(Trigger)
  (params (OverlappedComponent :type Primitive%20Component%20Object%20Reference) (OtherActor :type Actor%20Object%20Reference) (OtherComp :type Primitive%20Component%20Object%20Reference) (OtherBodyIndex :type Integer) (bFromSweep :type Boolean) (SweepResult :type Hit%20Result%20Structure%20%28by%20ref%29))
  (Utilities|Casting|CastToBP_Brian OtherActor)
  (CallFunction|ActivateFallingPlatform))

(event Custom|ActivateFallingPlatform
  (if (not (Variables|Default|GetActivated))
    (Variables|Default|SetActivated true)
    (Audio|PlaySoundatLocation (Variables|Default|GetSound) (Transformation|GetActorLocation) "0, 0, 0" 1.0 (Math|Random|RandomFloatinRange 9.5 1.05) 0.0 "/Game/Coding1/Audio/NewSoundAttenuation.NewSoundAttenuation" 0 0 0)
    (Rendering|Material|SetMaterial (Variables|Default|GetPlatform) 0 "/Game/Coding1/Materials/MI_Banana.MI_Banana")
    (Variables|Default|SetStart (Transformation|GetWorldTransform (Variables|Default|GetPlatform))) ; store the location we are at when activated
    (Development|PrintText "We will stay in the air for 1 second.")
    (Utilities|FlowControl|Delay 1.0)
    (CallFunction|StartFalling)))

(event Custom|StartFalling
  (Development|PrintText "We're gonna fall for 5 seconds")
  (Audio|PlaySoundatLocation (Variables|Default|GetSound) (Transformation|GetActorLocation) "0, 0, 0" 1.0 0.8 0.0 "/Game/Coding1/Audio/NewSoundAttenuation.NewSoundAttenuation" 0 0 0)
  (Rendering|Material|SetMaterial (Variables|Default|GetPlatform) 0 "/Game/Coding1/Materials/MI_Red.MI_Red")
  (Physics|SetSimulatePhysics (Variables|Default|GetPlatform) true)
  (Utilities|FlowControl|Delay 5.0)
  (CallFunction|ResetPlatform))

(event Custom|ResetPlatform
  (Development|PrintText "Returning to start")
  (Audio|PlaySoundatLocation (Variables|Default|GetSound) (Transformation|GetActorLocation) "0, 0, 0" 1.0 0.9 0.0 "/Game/Coding1/Audio/NewSoundAttenuation.NewSoundAttenuation" 0 0 0)
  (Rendering|Material|SetMaterial (Variables|Default|GetPlatform) 0 "/Game/Variant_Combat/Materials/MI_Box_Destroyed.MI_Box_Destroyed")
  (Physics|SetSimulatePhysics (Variables|Default|GetPlatform) false)
  (Variables|Default|SetEnd (Transformation|GetWorldTransform (Variables|Default|GetPlatform)))
  (bind _newtrack_0 (Timeline|ReturnToStart PlayFromStart)
    (:Update
      (Transformation|SetWorldTransform (Variables|Default|GetPlatform) (Math|Transform|Lerp(Transform) (Variables|Default|GetEnd) (Variables|Default|GetStart) _newtrack_0) false false))
    (:Finished
      (Development|PrintText "Platform is Reset")
      (Variables|Default|SetActivated false) ; platform is ready to be activated again
      (Rendering|Material|SetMaterial (Variables|Default|GetPlatform) 0 "/Game/LevelPrototyping/Materials/MI_DefaultColorway.MI_DefaultColorway")
      (Audio|PlaySoundatLocation (Variables|Default|GetSound) (Transformation|GetActorLocation) "0, 0, 0" 1.0 1.2 0.0 "/Game/Coding1/Audio/NewSoundAttenuation.NewSoundAttenuation" 0 0 0))))

(event EventBeginPlay)

(fn ConstructionScript)
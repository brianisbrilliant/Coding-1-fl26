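; BP_Banana is a pickup item that heals the player when used.
; Pickup stores the owner and disables the mesh's collision and physics, while Drop re-enables both and throws the banana forward with an impulse.
; Use adds health to the BP_Brian owner, asks its BPCInteract component to drop the banana, then destroys the actor after a short delay.
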(event EventUse
  (bind _asbp_brian (Utilities|Casting|CastToBP_Brian (Variables|Default|GetOwner_0)))
  (Variables|/Game/Coding1/Blueprints/BP_Brian.BP_Brian_C|SetHealth _asbp_brian (+ (Variables|/Game/Coding1/Blueprints/BP_Brian.BP_Brian_C|GetHealth _asbp_brian) 1e+01)) ; add 10 to the player's health.
  (Default|TrytoDrop (Variables|/Game/Coding1/Blueprints/BP_Brian.BP_Brian_C|GetBPC_Interact _asbp_brian))
  (Utilities|FlowControl|Delay 1.0)
  (Actor|DestroyActor))

(event EventDrop
  (bind _banana (Variables|Default|GetBanana))
  (Development|PrintText "Banana is being dropped" true true "(R=1.000000,G=0.002387,B=0.040085,A=1.000000)")
  (Collision|SetCollisionEnabled _banana "QueryAndPhysics")
  (Physics|SetSimulatePhysics _banana true)
  (Physics|AddImpulse _banana (* (Math|Vector|GetForwardVector _banana) 5e+02) "None" true))

(event EventPickup
  (params (Owner :type Actor%20Object%20Reference))
  (bind _banana (Variables|Default|GetBanana))
  (Variables|Default|SetOwner_0 Owner)
  (Development|PrintText "Banana is being picked up" true true "(R=0.000000,G=1.000000,B=0.125358,A=1.000000)")
  (Collision|SetCollisionEnabled _banana "NoCollision") ; make sure all other meshes have\ncollision turned off.
  (Physics|SetSimulatePhysics _banana false))

(fn ConstructionScript)
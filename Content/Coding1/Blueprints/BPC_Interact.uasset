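; BPC_Interact is a component for the BP_Brian player character that handles picking up, dropping and using items.
; Every tick, a camera-forward sphere trace stores any hit actor implementing BPI_Item as the in-focus item.
; E attaches that item to the left-hand socket if nothing is held, Q drops it, and left mouse uses it.
; Pickup, drop and use behavior is delegated to the item through interface messages.
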(event Custom|Looking
  (bind _as_bp_brian (Variables|Default|GetAs%20BP%20Brian))
  (bind _followcamera (Variables|/Game/Coding1/Blueprints/BP_Brian.BP_Brian_C|GetFollowCamera _as_bp_brian))
  (bind _returnvalue (Transformation|GetWorldLocation _followcamera))
  ;[0.002387 0.4327 1] Looking
  (bind _outhit (Collision|SphereTraceByChannel _returnvalue (+ _returnvalue (* (Math|Vector|GetForwardVector _followcamera) 5e+02)) 25.0 "TraceTypeQuery1" false (Utilities|Array|MakeArray _as_bp_brian) "None"))
  (if (Utilities|DoesObjectImplementInterface (.HitActor (Collision|BreakHitResult _outhit)) "/Game/Coding1/Blueprints/BPI_Item.BPI_Item_C")
    (Variables|Default|SetInFocusItem (.HitActor (Collision|BreakHitResult _outhit)))
    (else
      (Variables|Default|SetInFocusItem 0) ; clear the "in focus" item
    )))

(event Custom|Try%20to%20Drop
  ;[0.3112 1 0.002387] Drop
  (Class|BPIItem|Drop(Message) (Variables|Default|GetHeldItem))
  (Variables|Default|SetHeldItem 0) ; set helditem to nothing
)

(event EventBeginPlay
  ;[0.3417 0.001171 0.4906] Begin PLay
  (Utilities|FlowControl|Sequence
    (:then_1
      (bind _asbp_brian (Utilities|Casting|CastToBP_Brian (Components|GetOwner)))
      (Variables|Default|SetAs%20BP%20Brian _asbp_brian) ; store this reference for later.
      (Development|PrintText "BPC Interact is a child of BP_Brian"))))

(event EventTick
  (params (DeltaSeconds :type Float%20%28single-precision%29))
  ;[0.002387 0.4327 1] Looking
  (CallFunction|Looking))

(event Input|KeyboardEvents|Q
  (params (Key :type Key%20Structure :default "None"))
  ;[0.3112 1 0.002387] Drop
  (:Pressed
    (CallFunction|TrytoDrop)))

(event Input|KeyboardEvents|E
  (params (Key :type Key%20Structure :default "None"))
  ;[1 0.3563 0.002387] Pickup
  (:Pressed
    (bind _infocusitem (Variables|Default|GetInFocusItem) ; are we looking at something?
      (:then
        (Variables|Default|GetHeldItem ; are we holding something?
          (:then
            (Development|PrintText "we're already holding something"))
          (:else
            (bind _output_get (Variables|Default|SetHeldItem _infocusitem)) ; set heldItem to be the item\nwe are focusing on.
            (Transformation|AttachComponentToComponent _output_get (Variables|/Script/Engine.Character|GetMesh (Variables|Default|GetAs%20BP%20Brian)) "ik_hand_l" "SnapToTarget" "SnapToTarget" "KeepRelative" true) ; Move HeldItem to player's Hand
            (Class|BPIItem|Pickup(Message) (Variables|Default|GetHeldItem) (Variables|Default|GetAs%20BP%20Brian)))))
      (:else
        (Development|PrintText "We aren't looking at an item")))))

(event Input|MouseEvents|LeftMouseButton
  (params (Key :type Key%20Structure :default "None"))
  ;[1 0.002387 0.04009] Use
  (:Pressed
    (bind _helditem (Variables|Default|GetHeldItem)
      (:then
        (Class|BPIItem|Use(Message) _helditem))
      (:else))))
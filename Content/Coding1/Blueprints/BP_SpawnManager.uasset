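; A spawn manager that triggers three timed waves of increasing size across the level's BP_Spawner actors.
; BeginPlay gathers the spawners, then calls SpawnWave at intervals, which loops SpawnAThing for the requested count.
; SpawnAThing steps an index through the spawner array, reshuffling and resetting when it runs past the end.
; An AutoSpawn spawner advances the index before spawning; others spawn first, then re-trigger SpawnAThing after a delay.
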(event Custom|Spawn%20a%20thing
  (if (>= (Variables|Default|GetIndex) (Utilities|Array|Length (Variables|Default|GetSpawners))) ; are we at the end of our array?
    ;[0.15 0.15 0.15 0.5] re-shuffle the spawners and reset index
    (Utilities|Array|Shuffle (Variables|Default|GetSpawners))
    (Variables|Default|SetIndex 0))
  (if (Variables|/Game/Coding1/Blueprints/BP_Spawner.BP_Spawner_C|GetAuto-Spawn (Utilities|Array|Get(acopy) (Variables|Default|GetSpawners) (Variables|Default|GetIndex)))
    (Math|Integer|IncrementInt (Variables|Default|GetIndex)
      (:%20%20
        (Default|SpawnThing (Utilities|Array|Get(acopy) (Variables|Default|GetSpawners) (Variables|Default|GetIndex))) ; call the spawn function on the spawner
      ))
    (else
      (Default|SpawnThing (Utilities|Array|Get(acopy) (Variables|Default|GetSpawners) (Variables|Default|GetIndex))) ; call the spawn function on the spawner
      (Math|Integer|IncrementInt (Variables|Default|GetIndex)
        (:%20%20
          (Utilities|FlowControl|Delay 5.0) ; wait 5 seconds...
          (CallFunction|SpawnAThing))))))

(event Custom|Spawn%20Wave
  (params (Count :type Integer))
  (for _index (range 0 Count)
    (CallFunction|SpawnAThing)))

(event EventBeginPlay
  (bind _outactors (Actor|GetAllActorsOfClass "/Game/Coding1/Blueprints/BP_Spawner.BP_Spawner_C")) ; Get all the spawners
  (Variables|Default|SetSpawners _outactors)
  (CallFunction|SpawnWave 5)
  (Utilities|FlowControl|Delay 1e+01)
  (CallFunction|SpawnWave 15)
  (Utilities|FlowControl|Delay 1e+01)
  (CallFunction|SpawnWave 30))

(fn ConstructionScript)
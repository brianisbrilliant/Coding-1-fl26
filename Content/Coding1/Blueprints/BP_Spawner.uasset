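; BP_Spawner is a spawner actor that spawns a configurable class at its SpawnPoint transform, starting on BeginPlay when AutoSpawn is set.
; SpawnThing refuses colliding spawns and retries itself after a short delay until one succeeds.
; After a success, it schedules another spawn on a longer delay if AutoSpawn is on, otherwise it stops.
; Debug text prints on startup and on each attempt.
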(event Custom|Spawn%20Thing
  (Development|PrintText "Spawning the thing")
  (bind _returnvalue (Game|SpawnActorfromClass (Variables|Default|GetThing%20to%20Spawn) (Transformation|GetWorldTransform (Variables|Default|GetSpawn%20Point)) "DontSpawnIfColliding" "OverrideRootScale" 0 0))
  (Utilities|IsValid _returnvalue
    (:Is%20Valid
      (if (Variables|Default|GetAuto-Spawn)
        (Utilities|FlowControl|Delay 5.0)
        (CallFunction|SpawnThing :!label _label)))
    (:Is%20Not%20Valid
      (Utilities|FlowControl|Delay 0.5) ; keep trying to spawn until done.
      (goto _label))))

(event EventBeginPlay
  (Development|PrintText "Spawner active")
  (if (Variables|Default|GetAuto-Spawn)
    (CallFunction|SpawnThing)))

(fn ConstructionScript)